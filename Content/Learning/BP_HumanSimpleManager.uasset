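; Learning Agents manager that trains or runs a walking policy for BP_HumanSimple actors.
; BeginPlay makes the manager a tick prerequisite of every human, then builds interactor, policy, critic and RL trainer from neural network data assets, passing GameState to interactor and trainer.
; RunInference switches Tick between policy inference and training, and also resets each human at startup when set.
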(event EventBeginPlay
  (Utilities|FlowControl|Sequence
    (:then_0
      (bind _outactors (Actor|GetAllActorsOfClass "/Game/ThirdPerson/Blueprints/BP_HumanSimple.BP_HumanSimple_C"))
      (bind _output_get (Variables|Default|SetHumanActors _outactors))
      (Actor|Tick|AddTickPrerequisiteActor _output_get self))
    (:then_1
      (bind _returnvalue (Class|LearningAgentsInteractor|MakeInteractor (Variables|Core|GetManager) "/Game/Learning/BP_HumanSimpleWalkingInteractor.BP_HumanSimpleWalkingInteractor_C" "Human Interactor"))
      (bind _output_get_2 (Variables|Core|SetInteractor _returnvalue))
      (bind _asbp_game_state (Utilities|Casting|CastToBP_GameState (Game|GetGameState)))
      (Variables|/Game/Learning/BP_HumanSimpleWalkingInteractor.BP_HumanSimpleWalkingInteractor_C|SetGameState _output_get_2 _asbp_game_state))
    (:then_2
      (bind _returnvalue_2 (Class|LearningAgentsPolicy|MakePolicy (Variables|Core|GetManager) (Variables|Core|GetInteractor) "/Script/LearningAgents.LearningAgentsPolicy" "Human Policy" "/Game/Learning/DataAssets/DA_HumanSimpleEncoder.DA_HumanSimpleEncoder" "/Game/Learning/DataAssets/DA_HumanSimplePolicy.DA_HumanSimplePolicy" "/Game/Learning/DataAssets/DA_HumanSimpleDecoder.DA_HumanSimpleDecoder" true true true (Variables|Settings|GetPolicy%20Settings) 1234))
      (Variables|Core|SetPolicy _returnvalue_2))
    (:then_3
      (bind _returnvalue_3 (Class|LearningAgentsCritic|MakeCritic (Variables|Core|GetManager) (Variables|Core|GetInteractor) (Variables|Core|GetPolicy) "/Script/LearningAgents.LearningAgentsCritic" "Human Critic" "/Game/Learning/DataAssets/DA_HumanSimpleCritic.DA_HumanSimpleCritic" true (Variables|Settings|GetCritic%20Settings) 1234))
      (Variables|Core|SetCritic _returnvalue_3))
    (:then_4
      (bind _returnvalue_4 (Class|LearningAgentsTrainer|MakeTrainer (Variables|Core|GetManager) (Variables|Core|GetInteractor) (Variables|Core|GetPolicy) (Variables|Core|GetCritic) "/Game/Learning/BP_HumanSimpleWalkingRLTrainer.BP_HumanSimpleWalkingRLTrainer_C" "Human Trainer" (Variables|Settings|GetTrainer%20Settings)))
      (bind _output_get_3 (Variables|Core|SetTrainer _returnvalue_4))
      (bind _asbp_game_state_2 (Utilities|Casting|CastToBP_GameState (Game|GetGameState)))
      (Variables|/Game/Learning/BP_HumanSimpleWalkingRLTrainer.BP_HumanSimpleWalkingRLTrainer_C|SetGameState _output_get_3 _asbp_game_state_2))
    (:then_5
      (if (Variables|Default|GetRunInference)
        (for _array_element (Variables|Default|GetHumanActors)
          (Default|ResetState _array_element))))))

(event EventTick
  (params (DeltaSeconds :type Float%20%28single-precision%29))
  (if (Variables|Default|GetRunInference)
    (Class|LearningAgentsPolicy|RunInference (Variables|Core|GetPolicy) 1.0)
    (else
      (Class|LearningAgentsTrainer|RunTraining (Variables|Core|GetTrainer) (Variables|Settings|GetTrainer%20Training%20Settings) (Variables|Settings|GetTrainer%20Game%20Settings) (Variables|Settings|GetTrainer%20Path%20Settings) true true))))

(fn ConstructionScript)