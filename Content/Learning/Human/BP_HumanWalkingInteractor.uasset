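; Learning Agents interactor that lets a neural policy drive a physics-based BP_Human, observing a goal actor for walking.
; Observations combine the goal location relative to the agent, actor rotation, and per-joint relative location, rotation, angular velocity and height from the agent's current state.
; The action is an array of clamped floats, scaled and offset per joint into angular orientation targets on the head, torso, arm and leg physics constraints.
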(fn SpecifyAgentObservation
  (params (InObservationSchema :type Learning%20Agents%20Observation%20Schema%20Object%20Reference))
  (return (Class|LearningAgentsObservations|SpecifyStructObservation InObservationSchema (Utilities|Map|MakeMap "Goal Location Observation" (Class|LearningAgentsObservations|SpecifyLocationObservation InObservationSchema) "Global Actor Rotation" (Class|LearningAgentsObservations|SpecifyRotationObservation InObservationSchema) "Relative Joints Location" (Class|LearningAgentsObservations|SpecifyStaticArrayObservation InObservationSchema (Class|LearningAgentsObservations|SpecifyLocationObservation InObservationSchema) 13) "Relative Joints Rotation" (Class|LearningAgentsObservations|SpecifyStaticArrayObservation InObservationSchema (Class|LearningAgentsObservations|SpecifyRotationObservation InObservationSchema) 13) "Relative Joints Angular Velocity" (Class|LearningAgentsObservations|SpecifyStaticArrayObservation InObservationSchema (Class|LearningAgentsObservations|SpecifyVelocityObservation InObservationSchema) 14) "Joints Height" (Class|LearningAgentsObservations|SpecifyStaticArrayObservation InObservationSchema (Class|LearningAgentsObservations|SpecifyFloatObservation InObservationSchema) 14)))))

(fn GatherAgentObservation
  (params (InObservationObject :type Learning%20Agents%20Observation%20Object%20Object%20Reference) (AgentId :type Integer))
  (bind (_goallocationobservation _globalactorrotationobservation _relativejointslocation _getrelativejointsrotation _getrelativejointsangularvelocity _getjointsheight) (Observation|GetObservations InObservationObject AgentId))
  (return (Class|LearningAgentsObservations|MakeStructObservation InObservationObject (Utilities|Map|MakeMap "Goal Location Observation" _goallocationobservation "Global Actor Rotation" _globalactorrotationobservation "Relative Joints Location" _relativejointslocation "Relative Joints Rotation" _getrelativejointsrotation "Relative Joints Angular Velocity" _getrelativejointsangularvelocity "Joints Height" _getjointsheight))))

(fn GetGoalLocationObservation
  (params (ObservationObject :type Learning%20Agents%20Observation%20Object%20Object%20Reference%20%28by%20ref%29) (Goal :type Actor%20Object%20Reference%20%28by%20ref%29) (Relative%20Transform :type Transform%20%28by%20ref%29))
  (return (Class|LearningAgentsObservations|MakeLocationObservation ObservationObject (Transformation|GetActorLocation Goal) Relative%20Transform 1e+03 "LocationObservation" false 0)))

(fn GetGlobalActorRotationObservation
  (params (ObservationObject :type Learning%20Agents%20Observation%20Object%20Object%20Reference%20%28by%20ref%29) (GlobalActorRotation :type Rotator%20%28by%20ref%29))
  (return (Class|LearningAgentsObservations|MakeRotationObservation ObservationObject GlobalActorRotation "0, 0, 0" "RotationObservation" false 0)))

(fn GetRelativeJointsLocation
  (params (ObservationObject :type Learning%20Agents%20Observation%20Object%20Object%20Reference%20%28by%20ref%29) (Relative%20Joints%20Location :type Array%20of%20Vectors))
  (for _array_element Relative%20Joints%20Location
    (Utilities|Array|Add (LocalVariables|GetL_RelativeJointsLocaiton) (Class|LearningAgentsObservations|MakeLocationObservation ObservationObject _array_element (Math|Transform|MakeTransform "0, 0, 0" "0, 0, 0" "1.000000,1.000000,1.000000") 1.5e+02 "LocationObservation" false 0)))
  (return (Class|LearningAgentsObservations|MakeStaticArrayObservation ObservationObject (LocalVariables|GetL_RelativeJointsLocaiton))))

(fn GetRelativeJointsRotation
  (params (ObservationObject :type Learning%20Agents%20Observation%20Object%20Object%20Reference%20%28by%20ref%29) (RelativeJointsRotation :type Array%20of%20Rotators))
  (for _array_element RelativeJointsRotation
    (Utilities|Array|Add (LocalVariables|GetL_RelativeJointsRotation) (Class|LearningAgentsObservations|MakeRotationObservation ObservationObject _array_element "0, 0, 0" "RotationObservation" false 0)))
  (return (Class|LearningAgentsObservations|MakeStaticArrayObservation ObservationObject (LocalVariables|GetL_RelativeJointsRotation))))

(fn GetRelativeJointsAngularVelocity
  (params (ObservationObject :type Learning%20Agents%20Observation%20Object%20Object%20Reference%20%28by%20ref%29) (Joints%20Angular%20Velocity :type Array%20of%20Vectors))
  (for _array_element Joints%20Angular%20Velocity
    (Utilities|Array|Add (LocalVariables|GetL_RelativeJointsAngularVelocity) (Class|LearningAgentsObservations|MakeVelocityObservation ObservationObject _array_element (Math|Transform|MakeTransform "0, 0, 0" "0, 0, 0" "1.000000,1.000000,1.000000") 4.0 "VelocityObservation" false 0)))
  (return (Class|LearningAgentsObservations|MakeStaticArrayObservation ObservationObject (LocalVariables|GetL_RelativeJointsAngularVelocity))))

(fn GetJointsHeight
  (params (ObservationObject :type Learning%20Agents%20Observation%20Object%20Object%20Reference%20%28by%20ref%29) (Joints%20Height :type Array%20of%20Floats%20%28double-precision%29))
  (for _array_element Joints%20Height
    (Utilities|Array|Add (LocalVariables|GetL_JointsHeight) (Class|LearningAgentsObservations|MakeFloatObservation ObservationObject _array_element 1.5e+02 "FloatObservation" false 0)))
  (return (Class|LearningAgentsObservations|MakeStaticArrayObservation ObservationObject (LocalVariables|GetL_JointsHeight))))

(fn GetObservations
  (params (ObservationObject :type Learning%20Agents%20Observation%20Object%20Object%20Reference%20%28by%20ref%29) (AgentId :type Integer))
  (bind _returnvalue (Class|LearningAgentsManagerListener|GetAgent AgentId "/Game/ThirdPerson/Blueprints/BP_Human.BP_Human_C"))
  (bind (_globalactorrotation _relativejointslocation _relativejointsrotation _jointsangularvelocity _jointsheight) (Default|GetCurrentAgentState _returnvalue))
  (bind _goallocationobservation (Observation|GetGoalLocationObservation ObservationObject (Variables|/Game/Core/BP_GameState.BP_GameState_C|GetGoal (Variables|Default|GetGameState)) (Transformation|GetActorTransform _returnvalue)))
  (bind _globalactorrotationobservation (Observation|GetGlobalActorRotationObservation ObservationObject _globalactorrotation))
  (bind _relativejointslocation_2 (Observation|GetRelativeJointsLocation ObservationObject _relativejointslocation))
  (bind _getrelativejointsrotation (Observation|GetRelativeJointsRotation ObservationObject _relativejointsrotation))
  (bind _relativejointsangularvelocity (Observation|GetRelativeJointsAngularVelocity ObservationObject _jointsangularvelocity))
  (bind _jointsheight_2 (Observation|GetJointsHeight ObservationObject _jointsheight))
  (return _goallocationobservation _globalactorrotationobservation _relativejointslocation_2 _getrelativejointsrotation _relativejointsangularvelocity _jointsheight_2))

(fn SpecifyAgentAction
  (params (InActionSchema :type Learning%20Agents%20Action%20Schema%20Object%20Reference))
  (return (Class|LearningAgentsActions|SpecifyStaticArrayAction InActionSchema (Class|LearningAgentsActions|SpecifyFloatAction InActionSchema "Target Angle") 33 "Target Angles")))

(fn PerformAgentAction
  (params (InActionObject :type Learning%20Agents%20Action%20Object%20Object%20Reference) (InActionObjectElement :type Learning%20Agents%20Action%20Object%20Element%20Structure%20%28by%20ref%29) (AgentId :type Integer))
  (bind _outelements (Class|LearningAgentsActions|GetStaticArrayAction InActionObject InActionObjectElement "Target Angles"))
  (for _array_element _outelements
    (bind _outvalue (Class|LearningAgentsActions|GetFloatAction InActionObject _array_element 1.0 "Target Angle" false 0))
    (Utilities|Array|Add (LocalVariables|GetL_Actions) (Math|Float|Clamp(Float) _outvalue -2.0 2.0)))
  (Actions|SetAngularOrientationTargets (LocalVariables|GetL_Actions) AgentId)
  (return))

(fn SetAngularOrientationTargets
  (params (Actions :type Array%20of%20Floats%20%28double-precision%29) (AgentId :type Integer))
  (LocalVariables|SetL_Human (Class|LearningAgentsManagerListener|GetAgent AgentId "/Game/ThirdPerson/Blueprints/BP_Human.BP_Human_C"))
  (Actions|Perform|SetHeadConstraint (Utilities|Array|Get(acopy) Actions) (LocalVariables|GetL_Human))
  (Actions|Perform|SetBodyLegConstraintR (Utilities|Array|Get(acopy) Actions 1) (Utilities|Array|Get(acopy) Actions 2) (Utilities|Array|Get(acopy) Actions 3) (LocalVariables|GetL_Human))
  (Actions|Perform|SetBodyLegConstraintL (Utilities|Array|Get(acopy) Actions 4) (Utilities|Array|Get(acopy) Actions 5) (Utilities|Array|Get(acopy) Actions 6) (LocalVariables|GetL_Human))
  (Actions|Perform|SetThingLegConstraintR (Utilities|Array|Get(acopy) Actions 7) (Utilities|Array|Get(acopy) Actions 8) (LocalVariables|GetL_Human))
  (Actions|Perform|SetThingLegConstraintL (Utilities|Array|Get(acopy) Actions 9) (Utilities|Array|Get(acopy) Actions 10) (LocalVariables|GetL_Human))
  (Actions|Perform|SetLegFootConstraintR (Utilities|Array|Get(acopy) Actions 11) (Utilities|Array|Get(acopy) Actions 12) (Utilities|Array|Get(acopy) Actions 13) (LocalVariables|GetL_Human))
  (Actions|Perform|SetLegFootConstraintL (Utilities|Array|Get(acopy) Actions 14) (Utilities|Array|Get(acopy) Actions 15) (Utilities|Array|Get(acopy) Actions 16) (LocalVariables|GetL_Human))
  (Actions|Perform|SetBodyConstraint20 (Utilities|Array|Get(acopy) Actions 17) (Utilities|Array|Get(acopy) Actions 18) (Utilities|Array|Get(acopy) Actions 19) (LocalVariables|GetL_Human))
  (Actions|Perform|SetBodyConstraint21 (Utilities|Array|Get(acopy) Actions 20) (Utilities|Array|Get(acopy) Actions 21) (Utilities|Array|Get(acopy) Actions 22) (LocalVariables|GetL_Human))
  (Actions|Perform|SetUpperArmConstraintR (Utilities|Array|Get(acopy) Actions 23) (Utilities|Array|Get(acopy) Actions 24) (Utilities|Array|Get(acopy) Actions 25) (LocalVariables|GetL_Human))
  (Actions|Perform|SetUpperArmConstraintL (Utilities|Array|Get(acopy) Actions 26) (Utilities|Array|Get(acopy) Actions 27) (Utilities|Array|Get(acopy) Actions 28) (LocalVariables|GetL_Human))
  (Actions|Perform|SetLowerArmConstraintR (Utilities|Array|Get(acopy) Actions 29) (Utilities|Array|Get(acopy) Actions 30) (LocalVariables|GetL_Human))
  (Actions|Perform|SetLowerArmConstraintL (Utilities|Array|Get(acopy) Actions 31) (Utilities|Array|Get(acopy) Actions 32) (LocalVariables|GetL_Human)))

(fn SetHeadConstraint
  (params (RowAngle :type Float%20%28double-precision%29) (Human :type BP%20Human%20Object%20Reference%20%28by%20ref%29))
  (Class|PhysicsConstraintComponent|SetAngularOrientationTarget (Variables|/Game/ThirdPerson/Blueprints/BP_Human.BP_Human_C|GetHeadConstraint Human) (Math|Rotator|MakeRotator (* RowAngle 45.0) 0.0 0.0)))

(fn SetBodyLegConstraintR
  (params (Row :type Float%20%28double-precision%29) (Pitch :type Float%20%28double-precision%29) (Yaw :type Float%20%28double-precision%29) (Human :type BP%20Human%20Object%20Reference%20%28by%20ref%29))
  (Class|PhysicsConstraintComponent|SetAngularOrientationTarget (Variables|/Game/ThirdPerson/Blueprints/BP_Human.BP_Human_C|GetBodyLegConstraint_R Human) (Math|Rotator|MakeRotator (* Row 22.5) (* Pitch 22.5) (* Yaw 22.5))))

(fn SetBodyLegConstraintL
  (params (Row :type Float%20%28double-precision%29) (Pitch :type Float%20%28double-precision%29) (Yaw :type Float%20%28double-precision%29) (Human :type BP%20Human%20Object%20Reference%20%28by%20ref%29))
  (Class|PhysicsConstraintComponent|SetAngularOrientationTarget (Variables|/Game/ThirdPerson/Blueprints/BP_Human.BP_Human_C|GetBodyLegConstraint_L Human) (Math|Rotator|MakeRotator (* Row 22.5) (* Pitch 22.5) (* Yaw 22.5))))

(fn SetThingLegConstraintR
  (params (Pitch :type Float%20%28double-precision%29) (Yaw :type Float%20%28double-precision%29) (Human :type BP%20Human%20Object%20Reference%20%28by%20ref%29))
  (Class|PhysicsConstraintComponent|SetAngularOrientationTarget (Variables|/Game/ThirdPerson/Blueprints/BP_Human.BP_Human_C|GetThingLegConstraint_R Human) (Math|Rotator|MakeRotator 0.0 (* Pitch 2.5) (+ (* Yaw 22.5) 45.0))))

(fn SetThingLegConstraintL
  (params (Pitch :type Float%20%28double-precision%29) (Yaw :type Float%20%28double-precision%29) (Human :type BP%20Human%20Object%20Reference%20%28by%20ref%29))
  (Class|PhysicsConstraintComponent|SetAngularOrientationTarget (Variables|/Game/ThirdPerson/Blueprints/BP_Human.BP_Human_C|GetThingLegConstraint_L Human) (Math|Rotator|MakeRotator 0.0 (* Pitch 2.5) (+ (* Yaw 22.5) 45.0))))

(fn SetLegFootConstraintR
  (params (Row :type Float%20%28double-precision%29) (Pitch :type Float%20%28double-precision%29) (Yaw :type Float%20%28double-precision%29) (Human :type BP%20Human%20Object%20Reference%20%28by%20ref%29))
  (Class|PhysicsConstraintComponent|SetAngularOrientationTarget (Variables|/Game/ThirdPerson/Blueprints/BP_Human.BP_Human_C|GetLegFootConstraint_R Human) (Math|Rotator|MakeRotator (* Row 22.5) (* Pitch 22.5) (* Yaw 22.5))))

(fn SetLegFootConstraintL
  (params (Row :type Float%20%28double-precision%29) (Pitch :type Float%20%28double-precision%29) (Yaw :type Float%20%28double-precision%29) (Human :type BP%20Human%20Object%20Reference%20%28by%20ref%29))
  (Class|PhysicsConstraintComponent|SetAngularOrientationTarget (Variables|/Game/ThirdPerson/Blueprints/BP_Human.BP_Human_C|GetLegFootConstraint_L Human) (Math|Rotator|MakeRotator (* Row 22.5) (* Pitch 22.5) (* Yaw 22.5))))

(fn SetBodyConstraint20
  (params (Row :type Float%20%28double-precision%29%20%28by%20ref%29) (Pitch :type Float%20%28double-precision%29%20%28by%20ref%29) (Yaw :type Float%20%28double-precision%29%20%28by%20ref%29) (Human :type BP%20Human%20Object%20Reference%20%28by%20ref%29))
  (Class|PhysicsConstraintComponent|SetAngularOrientationTarget (Variables|/Game/ThirdPerson/Blueprints/BP_Human.BP_Human_C|GetBodyConstraint_02 Human) (Math|Rotator|MakeRotator (* Row 22.5) (* Pitch 5.0) (* Yaw 5.0))))

(fn SetBodyConstraint21
  (params (Row :type Float%20%28double-precision%29%20%28by%20ref%29) (Pitch :type Float%20%28double-precision%29%20%28by%20ref%29) (Yaw :type Float%20%28double-precision%29%20%28by%20ref%29) (Human :type BP%20Human%20Object%20Reference%20%28by%20ref%29))
  (Class|PhysicsConstraintComponent|SetAngularOrientationTarget (Variables|/Game/ThirdPerson/Blueprints/BP_Human.BP_Human_C|GetBodyConstraint_01 Human) (Math|Rotator|MakeRotator (* Row 22.5) (* Pitch 5.0) (* Yaw 5.0))))

(fn SetUpperArmConstraintR
  (params (Row :type Float%20%28double-precision%29%20%28by%20ref%29) (Pitch :type Float%20%28double-precision%29%20%28by%20ref%29) (Yaw :type Float%20%28double-precision%29%20%28by%20ref%29) (Human :type BP%20Human%20Object%20Reference%20%28by%20ref%29))
  (Class|PhysicsConstraintComponent|SetAngularOrientationTarget (Variables|/Game/ThirdPerson/Blueprints/BP_Human.BP_Human_C|GetUpperArmConstraint_R Human) (Math|Rotator|MakeRotator (* Row 22.5) (* Pitch 22.5) (* Yaw 22.5))))

(fn SetUpperArmConstraintL
  (params (Row :type Float%20%28double-precision%29%20%28by%20ref%29) (Pitch :type Float%20%28double-precision%29%20%28by%20ref%29) (Yaw :type Float%20%28double-precision%29%20%28by%20ref%29) (Human :type BP%20Human%20Object%20Reference%20%28by%20ref%29))
  (Class|PhysicsConstraintComponent|SetAngularOrientationTarget (Variables|/Game/ThirdPerson/Blueprints/BP_Human.BP_Human_C|GetUpperArmConstraint_L Human) (Math|Rotator|MakeRotator (* Row 22.5) (* Pitch 22.5) (* Yaw 22.5))))

(fn SetLowerArmConstraintR
  (params (Pitch :type Float%20%28double-precision%29%20%28by%20ref%29) (Yaw :type Float%20%28double-precision%29%20%28by%20ref%29) (Human :type BP%20Human%20Object%20Reference%20%28by%20ref%29))
  (Class|PhysicsConstraintComponent|SetAngularOrientationTarget (Variables|/Game/ThirdPerson/Blueprints/BP_Human.BP_Human_C|GetLowerArmConstraint_R Human) (Math|Rotator|MakeRotator 0.0 (* Pitch 2.5) (- (* Yaw 22.5) 45.0))))

(fn SetLowerArmConstraintL
  (params (Pitch :type Float%20%28double-precision%29%20%28by%20ref%29) (Yaw :type Float%20%28double-precision%29%20%28by%20ref%29) (Human :type BP%20Human%20Object%20Reference%20%28by%20ref%29))
  (Class|PhysicsConstraintComponent|SetAngularOrientationTarget (Variables|/Game/ThirdPerson/Blueprints/BP_Human.BP_Human_C|GetLowerArmConstraint_L Human) (Math|Rotator|MakeRotator 0.0 (* Pitch 2.5) (- (* Yaw 22.5) 45.0))))