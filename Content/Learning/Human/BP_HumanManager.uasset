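; Manager actor that sets up Learning Agents reinforcement learning for walking BP_Human actors.
; On BeginPlay it gathers the humans, makes them tick after itself, and builds interactor, policy, critic and trainer on the Human manager using saved neural network assets.
; The RunInference flag switches Tick between running the policy and running training, and also resets every human at startup when set.
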(event EventBeginPlay
  (Utilities|FlowControl|Sequence
    (:then_0
      (bind _outactors (Actor|GetAllActorsOfClass "/Game/ThirdPerson/Blueprints/BP_Human.BP_Human_C"))
      (bind _output_get (Variables|Default|SetHumanActors _outactors))
      (Actor|Tick|AddTickPrerequisiteActor _output_get self))
    (:then_1
      (bind _returnvalue (Class|LearningAgentsInteractor|MakeInteractor (Variables|Default|GetHuman) "/Game/Learning/Human/BP_HumanWalkingInteractor.BP_HumanWalkingInteractor_C" "Human Interactor"))
      (Variables|Core|SetInteractor _returnvalue))
    (:then_2
      (bind _returnvalue_2 (Class|LearningAgentsPolicy|MakePolicy (Variables|Default|GetHuman) (Variables|Core|GetInteractor) "/Script/LearningAgents.LearningAgentsPolicy" "Human Policy" "/Game/Learning/Human/DataAssets/Walking_5/DA_Human5WalkingEncoder.DA_Human5WalkingEncoder" "/Game/Learning/Human/DataAssets/Walking_5/DA_Human5WalkingPolicy.DA_Human5WalkingPolicy" "/Game/Learning/Human/DataAssets/Walking_5/DA_Human5WalkingDecoder.DA_Human5WalkingDecoder" true true true (Variables|Settings|GetPolicy%20Settings) 1000))
      (Variables|Core|SetPolicy _returnvalue_2))
    (:then_3
      (bind _returnvalue_3 (Class|LearningAgentsCritic|MakeCritic (Variables|Default|GetHuman) (Variables|Core|GetInteractor) (Variables|Core|GetPolicy) "/Script/LearningAgents.LearningAgentsCritic" "Human Critic" "/Game/Learning/Human/DataAssets/Walking_5/DA_Human5WalkingCritic.DA_Human5WalkingCritic" true (Variables|Settings|GetCritic%20Settings) 1000))
      (Variables|Core|SetCritic _returnvalue_3))
    (:then_4
      (bind _returnvalue_4 (Class|LearningAgentsTrainer|MakeTrainer (Variables|Default|GetHuman) (Variables|Core|GetInteractor) (Variables|Core|GetPolicy) (Variables|Core|GetCritic) "/Game/Learning/Human/BP_HumanWalkingRLTrainer.BP_HumanWalkingRLTrainer_C" "Human Trainer" (Variables|Settings|GetTrainer%20Settings)))
      (Variables|Core|SetTrainer _returnvalue_4))
    (:then_5
      (if (Variables|Default|GetRunInference)
        (for _array_element (Variables|Default|GetHumanActors)
          (Default|ResetState _array_element))))))

(event EventTick
  (params (DeltaSeconds :type Float%20%28single-precision%29))
  (if (Variables|Default|GetRunInference)
    (Class|LearningAgentsPolicy|RunInference (Variables|Core|GetPolicy) 1.0)
    (else
      (Class|LearningAgentsTrainer|RunTraining (Variables|Core|GetTrainer) (Variables|Settings|GetTrainer%20Training%20Settings) (Variables|Settings|GetTrainer%20Game%20Settings) (Variables|Settings|GetTrainer%20Path%20Settings) true true))))

(fn ConstructionScript)