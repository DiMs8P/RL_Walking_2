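; Learning Agents training environment for BP_Human walkers learning to reach the game state's Goal.
; Distance reward pays normalized XY progress or a flat penalty, and height reward scores head-over-body-over-feet posture.
; GatherAgentReward calls both, but their sums are unconnected, so it returns LResult unchanged, and height always checks agent 0.
; Episodes terminate near the goal or on timeout; resets restore agents, timer and origin-to-goal baseline distance.
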(fn GatherAgentReward
  (params (AgentId :type Integer))
  (bind _distancereward (Reward|GetDistanceReward AgentId))
  (bind _heightreward (Reward|GetHeightReward))
  (return (LocalVariables|GetL_Result)))

(fn GetHeightReward
  (params (AgentId :type Integer))
  (bind _returnvalue (Class|LearningAgentsManagerListener|GetAgent AgentId "/Game/ThirdPerson/Blueprints/BP_Human.BP_Human_C"))
  (bind _body_0 (Variables|/Game/ThirdPerson/Blueprints/BP_Human.BP_Human_C|GetBody_0 _returnvalue))
  (bind _returnvalue_2 (Transformation|GetWorldLocation _body_0))
  (if (> (.z (Transformation|GetWorldLocation (Variables|/Game/ThirdPerson/Blueprints/BP_Human.BP_Human_C|GetHead _returnvalue))) (.z _returnvalue_2))
    (Math|Float|IncrementFloat (LocalVariables|GetL_VerticalReward)
      (:%20%20
        _)))
  (if (and (> (.z _returnvalue_2) (.z (Transformation|GetWorldLocation (Variables|/Game/ThirdPerson/Blueprints/BP_Human.BP_Human_C|GetFoot_R _returnvalue)))) (> (.z _returnvalue_2) (.z (Transformation|GetWorldLocation (Variables|/Game/ThirdPerson/Blueprints/BP_Human.BP_Human_C|GetFoot_L _returnvalue)))))
    (Math|Float|IncrementFloat (LocalVariables|GetL_VerticalReward)
      (:%20%20
        _)))
  (return (LocalVariables|GetL_VerticalReward)))

(fn GetDistanceReward
  (params (AgentId :type Integer))
  ;[1 1 1] Reward for coming closer
  (LocalVariables|SetL_Reward (Math|Float|SelectFloat (Math|Float|Max(Float) 0.0 (Math|Float|SafeDivide (- (.Value (Utilities|Map|Find (Variables|Default|GetPreviousDistances) AgentId)) (Utils|GetDistancetoGoal AgentId)) (Variables|Default|GetInitialDistance))) -5.0 (> (.Value (Utilities|Map|Find (Variables|Default|GetPreviousDistances) AgentId)) (Utils|GetDistancetoGoal AgentId))))
  (Utilities|Map|Add (Variables|Default|GetPreviousDistances) AgentId (Utils|GetDistancetoGoal AgentId))
  (return (LocalVariables|GetL_Reward)))

(fn GetDistancetoGoal
  (params (AgentId :type Integer))
  (return (Math|Vector|VectorLengthXY (- (Transformation|GetActorLocation (Class|LearningAgentsManagerListener|GetAgent AgentId "/Game/ThirdPerson/Blueprints/BP_Human.BP_Human_C")) (Transformation|GetActorLocation (Variables|/Game/Core/BP_GameState.BP_GameState_C|GetGoal (Variables|Default|GetGameState)))))))

(fn GatherAgentCompletion
  (params (AgentId :type Integer))
  (bind _returnvalue (Complition|GetTimeComlition AgentId))
  (LocalVariables|SetL_TimeComplition _returnvalue)
  (bind _returnvalue_2 (Complition|GetRewardComplition AgentId))
  (LocalVariables|SetL_RewardComplition _returnvalue_2)
  (if (or (Utilities|Enum|Equal(Enum) (LocalVariables|GetL_TimeComplition) "Termination") (Utilities|Enum|Equal(Enum) (LocalVariables|GetL_RewardComplition) "Termination"))
    (return "Termination")
    (else
      (return "Running"))))

(fn ResetAgentEpisodes
  (params (AgentIds :type Array%20of%20Integers))
  (CallFunction|ResetState)
  (for _array_element AgentIds
    (CallFunction|ResetAgentEpisodeOverride _array_element))
  (return))

(fn ResetAgentEpisode
  (params (AgentId :type Integer))
  (Default|ResetState (Class|LearningAgentsManagerListener|GetAgent AgentId "/Game/ThirdPerson/Blueprints/BP_Human.BP_Human_C"))
  (Utilities|Map|Add (Variables|Default|GetPreviousDistances) AgentId (Variables|Default|GetInitialDistance)))

(fn ResetState
  (Variables|Default|SetInitialDistance (Math|Vector|VectorLengthXY (Transformation|GetActorLocation (Variables|/Game/Core/BP_GameState.BP_GameState_C|GetGoal (Variables|Default|GetGameState)))))
  (Variables|/Game/Core/BP_GameState.BP_GameState_C|SetTime (Variables|Default|GetGameState) 0.0))

(fn ResetAgentEpisodeOverride
  (params (AgentId :type Integer))
  (Default|ResetState (Class|LearningAgentsManagerListener|GetAgent AgentId "/Game/ThirdPerson/Blueprints/BP_Human.BP_Human_C"))
  (Utilities|Map|Add (Variables|Default|GetPreviousDistances) AgentId (Variables|Default|GetInitialDistance)))

(fn GetRewardComplition
  (params (AgentId :type Integer))
  (bind _return_value (Utils|GetDistancetoGoal AgentId))
  (bind _returnvalue (< _return_value 5e+01))
  (if _returnvalue
    (Development|PrintString self "Finished" true true "(R=1.000000,G=0.047313,B=0.000000,A=1.000000)"))
  (return (Class|LearningAgentsCompletions|MakeCompletiononCondition _returnvalue "Termination" "ConditionCompletion" false 0)))

(fn GetTimeComlition
  (params (AgentId :type Integer))
  (return (Class|LearningAgentsCompletions|MakeCompletiononTimeElapsed (Variables|/Game/Core/BP_GameState.BP_GameState_C|GetTime (Variables|Default|GetGameState)) 2e+01 "Termination" "TimeElapsedCompletion" false 0)))